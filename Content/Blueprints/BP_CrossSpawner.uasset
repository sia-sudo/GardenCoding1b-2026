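; BP_CrossSpawner is a cross item that the third-person character can pick up and use to spawn crosses.
; Overlap stores the character as Player and calls its TryToPickUpItem with itself.
; Pickup attaches the cross to the hand_r socket on the character's mesh.
; PrimaryAction spawns a BP_SingleCross at the item's transform, and Drop destroys the item, with each of the three actions printing debug text.
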(event `self.ReceiveActorBeginOverlap`
  (params (OtherActor :type "Actor Object Reference"))
  (bind _asbp_third_person_character (cast `/Game/ThirdPerson/Blueprints/BP_ThirdPersonCharacter` OtherActor))
  (set `self.Player` _asbp_third_person_character) ; Promote to variable
  (`/Game/ThirdPerson/Blueprints/BP_ThirdPersonCharacter.Try to pick up item` _asbp_third_person_character self))

(event `/Game/Blueprints/BPI_Item.Pickup`
  (`KismetSystemLibrary.PrintText` "The cross is getting picked up")
  (`self.K2_AttachToComponent` (`Character.Mesh` (`self.Player`)) "hand_r" "SnapToTarget" "SnapToTarget" "KeepRelative"))

(event `/Game/Blueprints/BPI_Item.Primary Action`
  (`KismetSystemLibrary.PrintText` "Hitting")
  (`|SpawnActorFromClass` "/Game/Blueprints/BP_SingleCross.BP_SingleCross_C" (`self.GetTransform`) "Undefined" "MultiplyWithRoot" null null))

(event `/Game/Blueprints/BPI_Item.Drop`
  (`KismetSystemLibrary.PrintText` "The cross is getting dropped")
  (`self.K2_DestroyActor`))

(fn `UserConstructionScript`)