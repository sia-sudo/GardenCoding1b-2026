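; BP_Door is a locked door that the player opens by spending a key.
; On actor overlap it casts to BP_ThirdPersonCharacter, prints a knocking message and checks the character's TotalKeys.
; With a key available, it decrements the count and destroys the Door and BoxCollision components, leaving the actor itself in place.
; Without a key, it prints a locked message.
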(event `self.ReceiveActorBeginOverlap`
  (params (OtherActor :type "Actor Object Reference"))
  (bind _asbp_third_person_character (cast `/Game/ThirdPerson/Blueprints/BP_ThirdPersonCharacter` OtherActor))
  (`KismetSystemLibrary.PrintText` "The player is knocking")
  (bind _totalkeys (`/Game/ThirdPerson/Blueprints/BP_ThirdPersonCharacter.TotalKeys` _asbp_third_person_character))
  (if (> _totalkeys 0)
    (`/Engine/EditorBlueprintResources/StandardMacros.DecrementInt` _totalkeys ; remove a key from totalkeys
      (:`  `
        (`ActorComponent.K2_DestroyComponent` (`self.Door`))
        (`ActorComponent.K2_DestroyComponent` (`self.BoxCollision`))))
    (else
      (`KismetSystemLibrary.PrintText` "Locked"))))

(fn `UserConstructionScript`)