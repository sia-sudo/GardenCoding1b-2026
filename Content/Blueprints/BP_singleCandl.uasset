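; Candle actor that picks a random static mesh at BeginPlay and gradually shrinks to simulate burning down.
; A self-repeating loop, capped at 19 passes by a DoN node, waits a random few seconds, then calls BurnOut to subtract a random amount from the mesh scale.
; Each pass also sets AutoDestroyWhenFinished and checks the DoN counter, enabling query and physics collision with a debug print if it equals zero.
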(event `self.ReceiveBeginPlay`
  (`StaticMeshComponent.SetStaticMesh` (`self.SM_singlecandle`) (`KismetArrayLibrary.Array_Random` (`self.New Mesh`)))
  (`self.The burn out loop`))

(event `The burn out loop`
  (bind _counter (`/Engine/EditorBlueprintResources/StandardMacros.Do N` 19 :!label _label)
    (:`Exit`
      (`KismetSystemLibrary.Delay` (`KismetMathLibrary.RandomFloatInRange` 5.0 7.0))
      (`self.Burn out`)
      (set `self.bAutoDestroyWhenFinished` true)
      (if (== _counter 0)
        (`PrimitiveComponent.SetCollisionEnabled` (`self.SM_singlecandle`) "QueryAndPhysics")
        (`KismetSystemLibrary.PrintText` "Collision Enabled!")
        (else
          (goto _label))))))

(event `Burn out`
  (bind _sm_singlecandle (`self.SM_singlecandle`))
  (`SceneComponent.SetRelativeScale3D` _sm_singlecandle (- (`SceneComponent.RelativeScale3D` _sm_singlecandle) (`KismetMathLibrary.RandomFloatInRange` 0.05 0.1))))

(fn `UserConstructionScript`)