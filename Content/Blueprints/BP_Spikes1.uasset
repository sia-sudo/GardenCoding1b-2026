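; Spike trap hazard that moves vertically like a piston and sends the third-person character back to its checkpoint on overlap.
; On BeginPlay a timeline starts from a small random time offset, so the start phase varies per instance.
; Its track drives a Lerp on the spikes' relative Z, and an Impact event plays an attenuated sound at the actor's location.
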(event `self.ReceiveBeginPlay`
  (`|ExecutionSequence`
    (:`then_0`
      (bind (_direction _verticalspikeslocation) (`Timeline|Timeline` :`NewTime` (`KismetMathLibrary.RandomFloatInRange` 0.0 0.5) :!via `SetNewTime` :!label _label)
        (:`Update`
          (`SceneComponent.K2_SetRelativeLocation` (`self.Spikes_1`) (`KismetMathLibrary.MakeVector` 0.0 0.0 (`KismetMathLibrary.Lerp` -30.0 20.0 _verticalspikeslocation)) false false) ; Right-click the new location>slipt struck pin
        )
        (:`impact`
          (`GameplayStatics.PlaySoundAtLocation` "/Engine/EditorSounds/GamePreview/PossessPlayer.PossessPlayer" (`self.K2_GetActorLocation`) (struct) 1.0 1.0 0.0 "/Game/Audio/ATT_DefaultSpikes.ATT_DefaultSpikes" null null null))))
    (:`then_1`
      (goto _label))))

(event `self.Spikes_1.OnComponentBeginOverlap`
  (params (OverlappedComponent :type "PrimitiveComponent Object Reference") (OtherActor :type "Actor Object Reference") (OtherComp :type "PrimitiveComponent Object Reference") (OtherBodyIndex :type Integer) (bFromSweep :type Boolean) (SweepResult :type "HitResult Structure (by ref)"))
  (bind _asbp_third_person_character (cast `/Game/ThirdPerson/Blueprints/BP_ThirdPersonCharacter` OtherActor))
  (`/Game/ThirdPerson/Blueprints/BP_ThirdPersonCharacter.ResetToCheckpoint` _asbp_third_person_character))

(fn `UserConstructionScript`)