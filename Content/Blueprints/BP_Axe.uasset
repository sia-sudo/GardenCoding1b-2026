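; BP_Axe is an axe item that the third-person character can pick up on overlap.
; Overlap stores the character as Player and passes the axe to its TryToPickUpItem.
; Pickup attaches the axe to the hand_r socket on the player's mesh, and Drop destroys the actor instead of releasing it into the world.
; PrimaryAction only prints a message, as a placeholder with no gameplay effect.
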(event `self.ReceiveActorBeginOverlap`
  (params (OtherActor :type "Actor Object Reference"))
  (bind _asbp_third_person_character (cast `/Game/ThirdPerson/Blueprints/BP_ThirdPersonCharacter` OtherActor))
  (set `self.Player` _asbp_third_person_character)
  (`/Game/ThirdPerson/Blueprints/BP_ThirdPersonCharacter.Try to pick up item` _asbp_third_person_character self))

(event `/Game/Blueprints/BPI_Item.Pickup`
  (`KismetSystemLibrary.PrintText` "The axe is getting picked up")
  (`self.K2_AttachToComponent` (`Character.Mesh` (`self.Player`)) "hand_r" "SnapToTarget" "SnapToTarget" "KeepRelative"))

(event `/Game/Blueprints/BPI_Item.Primary Action`
  (`KismetSystemLibrary.PrintText` "I have an axe"))

(event `/Game/Blueprints/BPI_Item.Drop`
  (`KismetSystemLibrary.PrintText` "The axe is getting dropped")
  (`self.K2_DestroyActor`))

(fn `UserConstructionScript`)